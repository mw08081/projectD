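; BP_ProjectD_DefaultGameMode is the default game mode for ProjectD and owns the level's background music.
; On BeginPlay it caches BP_GameInstance, then InitBGM starts WV_bgm on its BGMPlayer at the volume stored in the game instance.
; Pitch is set once from global time dilation at start.
; ChangeBGMPlayerVolume exposes runtime adjustment of the music volume.
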(event EventBeginPlay
  (Development|PrintString "GameMode Init")
  (bind _asbp_game_instance (Utilities|Casting|CastToBP_GameInstance (Game|GetGameInstance)))
  (Variables|Default|SetBP_GameInstance _asbp_game_instance)
  (CallFunction|InitBGM))

(event EventTick
  (params (DeltaSeconds :type Float%20%28single-precision%29)))

(fn ConstructionScript)

(fn InitBGM
  (bind _bgm_player (Variables|Default|GetBGM_Player))
  (Audio|Components|Audio|SetSound _bgm_player "/Game/System/Sound/BGM/WV_bgm.WV_bgm")
  (Audio|Components|Audio|SetVolumeMultiplier _bgm_player (Variables|/Game/System/Manager/BP_GameInstance.BP_GameInstance_C|GetBGM (Variables|Default|GetBP_GameInstance)) :!class /Script/Engine.AudioComponent)
  (Audio|Components|Audio|SetPitchMultiplier _bgm_player (Class|GameplayStatics|GetGlobalTimeDilation))
  (Audio|Components|Audio|Play _bgm_player 0.0))

(fn ChangeBGMPlayerVolume
  (params (value :type Float%20%28double-precision%29))
  (Audio|Components|Audio|SetVolumeMultiplier (Variables|Default|GetBGM_Player) value :!class /Script/Engine.AudioComponent))