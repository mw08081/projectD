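; Helper actor that supplies Tick-driven timing for the slow-motion state and its cooldown held in BP_GameInstance.
; Each Tick accumulates elapsed time, then ends the slow and later the cooldown when their durations pass, both measured from the slow's start.
; It raises its own CustomTimeDilation during the slow, and writes flags and normal global time dilation back to the GameInstance.
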(event EventBeginPlay
  (bind _asbp_game_instance (Utilities|Casting|CastToBP_GameInstance (Game|GetGameInstance)))
  (Variables|Default|SetGameInstance _asbp_game_instance))

(event Collision|EventActorBeginOverlap
  (params (OtherActor :type Actor%20Object%20Reference)))

(event EventTick
  (params (DeltaSeconds :type Float%20%28single-precision%29))
  (Utilities|FlowControl|Sequence
    (:then_0
      (Variables|Default|SetElapsedTime (+ DeltaSeconds (Variables|Default|GetElapsedTime))))
    (:then_1
      (Slow|TickforIsinSlow)
      (Slow|TickforIsinSlowCooldown))))

(fn ConstructionScript)

(fn SetSlowStartTime
  (if (not (Variables|Slow|GetcanTickForIsInSlow))
    (Variables|Slow|SetslowStartTime (Variables|Default|GetElapsedTime))
    (Variables|Slow|SetcanTickForIsInSlow true)
    (CallFunction|SetCustomTimeDilation 4.0)))

(fn TickforIsinSlow
  (bind _gameinstance (Variables|Default|GetGameInstance))
  (if (Variables|/Game/System/Manager/BP_GameInstance.BP_GameInstance_C|GetisInSlow (Variables|Default|GetGameInstance))
    (Slow|SetSlowStartTime)
    (if (and (> (Variables|Default|GetElapsedTime) (+ (Variables|Slow|GetslowStartTime) (Variables|/Game/System/Manager/BP_GameInstance.BP_GameInstance_C|GetDURATION_SLOW (Variables|Default|GetGameInstance)))) (Variables|Slow|GetcanTickForIsInSlow))
      ;[1 1 1] For GameInstance Setting
      (Default|SetIsinSlow _gameinstance false)
      (Default|SetGlobalTimeDilation _gameinstance 1.0)
      (Variables|/Game/System/Manager/BP_GameInstance.BP_GameInstance_C|SetisInSlowCooldown (Variables|Default|GetGameInstance) true)
      ;[1 1 1] For GameInstanceTickHelper Setting
      (Variables|Slow|SetcanTickForIsInSlow false)
      (CallFunction|SetCustomTimeDilation 1.0)
      (Variables|Slow|SetcanTickForIsInSlowCooldown true))))

(fn SetCustomTimeDilation
  (params (_customTimeDilation :type Float%20%28double-precision%29))
  (Variables|Default|SetCustomTimeDilation _customTimeDilation))

(fn TickforIsinSlowCooldown
  (bind _gameinstance (Variables|Default|GetGameInstance))
  (if (Variables|Slow|GetcanTickForIsInSlowCooldown)
    (if (> (Variables|Default|GetElapsedTime) (+ (Variables|Slow|GetslowStartTime) (Variables|/Game/System/Manager/BP_GameInstance.BP_GameInstance_C|GetDURATION_SLOW_COOLDOWN (Variables|Default|GetGameInstance))))
      ;[1 1 1] For GameInstance Setting
      (Default|SetIsinSlowCooldown _gameinstance false)
      (Default|SetGlobalTimeDilation _gameinstance 1.0)
      ;[1 1 1] For GameInstanceTickHelper Setting
      (Variables|Slow|SetcanTickForIsInSlowCooldown false))))