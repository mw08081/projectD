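; Manager Blueprint that listens for Chaos physics collision and break events on a list of Geometry Collection actors.
; On BeginPlay it binds both events on each collection's component.
; Collisions draw a brief debug box at the impact point, while the break handler is empty.
; Unconnected leftover logic would debounce breaks through BP_FractureObject's FractureManageComponent, play a sound and zero the piece's velocity.
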(event Custom|GeometryCollectionCollisionEvent
  (params (CollisionInfo :type Chaos%20Physics%20Collision%20Info%20Structure%20%28by%20ref%29))
  (Rendering|Debug|DrawDebugBox (.location CollisionInfo) "3.000000,3.000000,3.000000" "(R=1.000000,G=0.008526,B=0.000000,A=1.000000)" "0, 0, 0" 1.0 0.0))

(event Custom|GeometryCollectionBreakEvnet
  (params (BreakEvent :type Chaos%20Break%20Event%20Structure%20%28by%20ref%29)))

(event EventBeginPlay
  (for _array_element (Variables|Default|GetGeometryCollections)
    (EventDispatchers|BindEventtoOnChaosPhysicsCollision (Variables|/Game/Prop/_Base_FractureObject/BP_FractureObject.BP_FractureObject_C|GetGeometryCollection _array_element) (EventDispatchers|CreateEvent :!event Custom|GeometryCollectionCollisionEvent))
    (EventDispatchers|BindEventtoOnChaosBreakEvent (Variables|/Game/Prop/_Base_FractureObject/BP_FractureObject.BP_FractureObject_C|GetGeometryCollection _array_element) (EventDispatchers|CreateEvent :!event Custom|GeometryCollectionBreakEvnet))))

(fn ConstructionScript)