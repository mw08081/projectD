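; BP_Bat is the player's bat weapon actor, turning mesh hits into blow effects for its owning BP_Hana, assigned through SetOwnerWithCasting.
; When Hana flags a blow effect, a hit spawns a Niagara effect at the impact point via the GameInstance and triggers GameMode slow time dilation.
; Otherwise, hits passing Hana's stack checks spawn a different effect, update her blow count and clear her can-stack flag.
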(event OnComponentHit(StaticMesh)
  (params (HitComponent :type Primitive%20Component%20Object%20Reference) (OtherActor :type Actor%20Object%20Reference) (OtherComp :type Primitive%20Component%20Object%20Reference) (NormalImpulse :type Vector :default "0, 0, 0") (Hit :type Hit%20Result%20Structure%20%28by%20ref%29))
  (bind _impactpoint (Collision|BreakHitResult Hit))
  (bind _myownerhana (Variables|Default|GetMyOwnerHana))
  (bind _bp_gameinstance (Variables|Default|GetBP_GameInstance))
  (bind _bp_gameinstance_2 (Variables|Default|GetBP_GameInstance))
  (bind _myownerhana_2 (Variables|Default|GetMyOwnerHana))
  (if (Variables|/Game/player/BP_Hana.BP_Hana_C|GetshouldPlayBlowNs _myownerhana_2)
    ;[1 1 1] Blow Ns
    (bind _ns (Default|GetNsfromENSCode _bp_gameinstance_2 "NewEnumerator9"))
    (Default|SpawnNsatLocation _bp_gameinstance_2 _ns _impactpoint)
    (Class|ProjectDDefaultGameMode|SlowTimedilation (Variables|Default|GetBP_GameMode))
    (else
      (bind _canstackblow (Default|CheckConditonCanStackBlowCnt _myownerhana_2 OtherActor))
      (if (and (Variables|/Game/player/BP_Hana.BP_Hana_C|GetcanStackBlowCnt _myownerhana_2) _canstackblow)
        (bind _ns_2 (Default|GetNsfromENSCode _bp_gameinstance "NewEnumerator0"))
        (Default|SpawnNsatLocation _bp_gameinstance _ns_2 _impactpoint)
        (Default|ManageBlowCnt _myownerhana false)
        (Default|SetCanStackBlowCnt _myownerhana false)))))

(event EventBeginPlay
  (bind _asbp_game_instance (Utilities|Casting|CastToBP_GameInstance (Game|GetGameInstance)))
  (Variables|Default|SetBP_GameInstance _asbp_game_instance)
  (bind _asbp_project_d_default_game_mode (Utilities|Casting|CastToBP_ProjectD_DefaultGameMode (Game|GetGameMode)))
  (Variables|Default|SetBP_GameMode _asbp_project_d_default_game_mode))

(event Collision|EventActorBeginOverlap
  (params (OtherActor :type Actor%20Object%20Reference)))

(event EventTick
  (params (DeltaSeconds :type Float%20%28single-precision%29)))

(fn ConstructionScript)

(fn SetOwnerwithCasting
  (params (Owner :type Actor%20Object%20Reference))
  (Actor|SetOwner Owner)
  (bind _asbp_hana (Utilities|Casting|CastToBP_Hana (Components|GetOwner)))
  (Variables|Default|SetMyOwnerHana _asbp_hana))