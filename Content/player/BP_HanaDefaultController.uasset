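; BP_HanaDefaultController is a player controller that sets up the in-game HUD and handles pausing.
; On BeginPlay it creates WB_Ingame, adds it to the viewport and stores the reference.
; Q toggles pause: pausing opens WB_Option_Ingame with the cursor and Game-and-UI input.
; Unpausing hides the cursor, restores game-only input and removes top-level widgets found by the WB_Option class, rather than a stored reference.
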(event EventBeginPlay
  (CallFunction|InitIngameWB))

(event EventTick
  (params (DeltaSeconds :type Float%20%28single-precision%29)))

(event Input|KeyboardEvents|Q
  (params (Key :type Key%20Structure :default "None"))
  (bind _returnvalue (Game|GetPlayerController 0))
  (:Pressed
    (if (Game|IsGamePaused)
      (Game|SetGamePaused false)
      (Variables|/Script/Engine.PlayerController|SetbShowMouseCursor (Game|GetPlayerController 0) false)
      (Input|SetInputModeGameOnly 0 false)
      (bind _foundwidgets (Widget|GetAllWidgetsOfClass "/Game/System/WidetBlueprint/WB_Option.WB_Option_C" true))
      (Widget|RemovefromParent _foundwidgets)
      (else
        (Game|SetGamePaused true)
        (bind _returnvalue_2 (UserInterface|CreateWidget "/Game/System/WidetBlueprint/WB_Option_Ingame.WB_Option_Ingame_C"))
        (UserInterface|Viewport|AddtoViewport _returnvalue_2 0)
        (Variables|/Script/Engine.PlayerController|SetbShowMouseCursor _returnvalue true)
        (Input|SetInputModeGameandUI _returnvalue 0 "DoNotLock" true false)))))

(fn ConstructionScript)

(fn InitIngameWB
  (bind _returnvalue (UserInterface|CreateWidget "/Game/System/WidetBlueprint/WB_Ingame.WB_Ingame_C"))
  (UserInterface|Viewport|AddtoViewport _returnvalue 0)
  (Variables|Default|SetWB_Ingame _returnvalue))