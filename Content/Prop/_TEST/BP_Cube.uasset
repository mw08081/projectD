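; Test cube prop for experimenting with impact force readouts from its static mesh's mass and velocity.
; Tick stores delta time and checks whether the cube is moving, but that branch leads nowhere.
; A disconnected debug print derives acceleration from velocity change, converts centimeters to meters, and multiplies by mass and delta time, labeling the result newtons.
; The previous-velocity update is also disconnected, and the construction script only calls its parent.
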(event EventBeginPlay
  (|CallParentFunction) ; This node is disabled and will not be called.\nDrag off pins to build functionality.
)

(event Collision|EventActorBeginOverlap
  (params (OtherActor :type Actor%20Object%20Reference))
  (|CallParentFunction OtherActor) ; This node is disabled and will not be called.\nDrag off pins to build functionality.
)

(event EventTick
  (params (DeltaSeconds :type Float%20%28single-precision%29))
  (|CallParentFunction DeltaSeconds)
  (Variables|Default|SetDt DeltaSeconds)
  (if (> (Math|Vector|VectorLength (Transformation|GetVelocity)) 0.1)
    _))

(fn ConstructionScript
  (|CallParentFunction))