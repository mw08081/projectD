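; Test prop actor that launches nearby level objects along its arrow a target distance based on their mass.
; Shortly after BeginPlay it runs a debug-drawn sphere trace at its location and handles each actor with an LvObjectRoot once.
; Mass feeds bat or non-bat range curves, giving initial speed and impulse, which it prints.
; Fracturing objects use GCMass and get an extra-scaled impulse on their Geometry Collection.
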(event EventBeginPlay
  (bind _returnvalue (Transformation|GetActorLocation))
  (Utilities|FlowControl|Delay 0.1)
  (bind _outhits (Collision|MultiSphereTraceByChannel _returnvalue _returnvalue 3e+01 "TraceTypeQuery1" false 0 "ForDuration"))
  (for _array_element _outhits
    (if (and (!= (Actor|GetComponentbyClass (.HitActor (Collision|BreakHitResult _array_element)) "/Script/ProjectD.LvObjectRoot") 0) (not (Utilities|Array|ContainsItem (Variables|Default|GetTracedActorList) (.HitActor (Collision|BreakHitResult _array_element)))))
      (Utilities|Array|Add (Variables|Default|GetTracedActorList) (.HitActor (Collision|BreakHitResult _array_element)))
      (bind _output_get (Variables|Default|SetIsFracture (Utilities|Enum|Equal(Enum) (Variables|/Script/ProjectD.LvObjectRoot|GetobjectType (Actor|GetComponentbyClass (.HitActor (Collision|BreakHitResult _array_element)) "/Script/ProjectD.LvObjectRoot")) "FracturingObject")))
      (if _output_get
        (bind _output_get_2 (Variables|TracedObject|SetcurTracedActor (.HitActor (Collision|BreakHitResult _array_element))))
        (bind _asbp_fracture_object (Utilities|Casting|CastToBP_FractureObject _output_get_2))
        (Variables|TracedObject|SetcurTracedPrimitiveComp (Variables|/Game/Prop/_Base/BP_FractureObject.BP_FractureObject_C|GetGeometryCollection _asbp_fracture_object))
        (Variables|Default|Setmass (* (Variables|/Game/Prop/_Base/BP_FractureObject.BP_FractureObject_C|GetGC_Mass _asbp_fracture_object) 1.0))
        (else
          (Variables|TracedObject|SetcurTracedActor (.HitActor (Collision|BreakHitResult _array_element)))
          (Variables|TracedObject|SetcurTracedPrimitiveComp (.HitComponent (Collision|BreakHitResult _array_element)))
          (Variables|Default|Setmass (Physics|GetMass (Variables|TracedObject|GetcurTracedPrimitiveComp)))))
      (if (Variables|Default|GetisBat)
        (Variables|Default|Setdist (* (Math|Float|Power 0.5 (Variables|Default|Getmass)) 42.87))
        (else
          ;[1 1 1] 사거리
          (if (> (Variables|Default|Getmass) 1.5)
            (Variables|Default|Setdist (* (Math|Float|Power 0.7368 (Variables|Default|Getmass)) 9.2101))
            (else
              (Variables|Default|Setdist (+ (* (Variables|Default|Getmass) -1e+01) 21.0))))))
      (Development|PrintString (Utilities|String|Append (Utilities|GetObjectName (Variables|TracedObject|GetcurTracedActor)) " will go" (Utilities|String|ToString(Float) (Variables|Default|Getdist)) "m" "(초기속도: " (Utilities|String|ToString(Float) (Math|Float|Sqrt (* (Variables|Default|Getdist) 1e+01))) "m/s)" "+ Impulse Scale: " (Utilities|String|ToString(Float) (* (Variables|Default|Getmass) (Math|Float|Sqrt (* (Variables|Default|Getdist) 1e+01)) 1e+02))))
      (Class|PrimitiveComponent|WakeRigidBody (Variables|TracedObject|GetcurTracedPrimitiveComp) "None")
      (if (Variables|Default|GetIsFracture)
        (Physics|AddImpulse (Variables|TracedObject|GetcurTracedPrimitiveComp) (* (* (Math|Vector|GetForwardVector (Variables|Default|GetArrow)) (* (Variables|Default|Getmass) (Math|Float|Sqrt (* (Variables|Default|Getdist) 1e+01)) 1e+02)) 21.0) "None" false)
        (else
          (Physics|AddImpulse (Variables|TracedObject|GetcurTracedPrimitiveComp) (* (Math|Vector|GetForwardVector (Variables|Default|GetArrow)) (* (Variables|Default|Getmass) (Math|Float|Sqrt (* (Variables|Default|Getdist) 1e+01)) 1e+02)) "None" false))))))

(event Collision|EventActorBeginOverlap
  (params (OtherActor :type Actor%20Object%20Reference)))

(event EventTick
  (params (DeltaSeconds :type Float%20%28single-precision%29)))

(fn ConstructionScript)