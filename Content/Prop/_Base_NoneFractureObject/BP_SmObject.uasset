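; Non-fractured prop base that can be grabbed and swaps to a damaged mesh when struck by a strong destruction field.
; On BeginPlay it passes its static mesh and mass to GrabManageComponent.
; Overlapping a MasterField or DelayMasterField whose strain exceeds the damage threshold converts it once.
; Conversion separately draws random meshes from the destroyed-mesh array for the displayed and grabbed meshes, so the two can differ.
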(event OnComponentBeginOverlap(StaticMesh)
  (params (OverlappedComponent :type Primitive%20Component%20Object%20Reference) (OtherActor :type Actor%20Object%20Reference) (OtherComp :type Primitive%20Component%20Object%20Reference) (OtherBodyIndex :type Integer) (bFromSweep :type Boolean) (SweepResult :type Hit%20Result%20Structure%20%28by%20ref%29))
  (bind _destroyed_tartget_staticmesh (Variables|CONST|GetDESTROYED_TARTGET_STATICMESH))
  (bind _outitem (Utilities|Array|Random _destroyed_tartget_staticmesh))
  (if (not (Variables|STATE|GetisConverted))
    (bind _asbp_master_field (Utilities|Casting|CastToBP_MasterField OtherActor)
      (:then
        (if (> (Variables|/Game/Prop/_FiledSystem/BP_MasterField.BP_MasterField_C|GetStrain%20Magnitude _asbp_master_field) (Variables|Const|GetDMG_THRESHOLD))
          (Variables|STATE|SetisConverted true :!label _label)
          (if (> (Utilities|Array|Length _destroyed_tartget_staticmesh) 0)
            (Components|StaticMesh|SetStaticMesh (Variables|Default|GetStaticMesh) _outitem)
            (Variables|/Game/Prop/_Base_Component/GrabManageComponent.GrabManageComponent_C|SetGrabbedStaticMesh (Variables|Default|GetGrabManageComponent) _outitem))))
      (:CastFailed
        (bind _asbp_delay_master_field (Utilities|Casting|CastToBP_DelayMasterField OtherActor))
        (if (> (Variables|/Game/Prop/_FiledSystem/BP_DelayMasterField.BP_DelayMasterField_C|GetStrain%20Magnitude _asbp_delay_master_field) (Variables|Const|GetDMG_THRESHOLD))
          (goto _label))))))

(event EventBeginPlay
  (bind _grabmanagecomponent (Variables|Default|GetGrabManageComponent))
  (bind _staticmesh (Variables|Default|GetStaticMesh))
  (Variables|/Game/Prop/_Base_Component/GrabManageComponent.GrabManageComponent_C|SetGrabbedStaticMesh _grabmanagecomponent (Variables|/Script/Engine.StaticMeshComponent|GetStaticMesh _staticmesh))
  (Variables|/Game/Prop/_Base_Component/GrabManageComponent.GrabManageComponent_C|SetGrabbedObjectMass _grabmanagecomponent (Physics|GetMass _staticmesh)))

(fn ConstructionScript)