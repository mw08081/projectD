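; Base fracturable prop that plays sound and effects when its Geometry Collection breaks.
; BeginPlay binds Chaos collision and break events and passes the collection mass to GrabManageComponent; the collision handler is empty.
; Every break plays the FractureManageComponent's sound code through BP_GameInstance.
; The first break also disables grabbing, marks it fractured, spawns its Niagara effect and calls EventDestroy on the game instance.
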(event Custom|ChaosCollisionEvent
  (params (CollisionInfo :type Chaos%20Physics%20Collision%20Info%20Structure%20%28by%20ref%29)))

(event Custom|ChaosBreakEvent
  (params (BreakEvent :type Chaos%20Break%20Event%20Structure%20%28by%20ref%29))
  (bind _asbp_game_instance (Utilities|Casting|CastToBP_GameInstance (Game|GetGameInstance)))
  (Default|SpawnSoundatLocation _asbp_game_instance (.location BreakEvent) (Variables|/Game/Prop/_Base_Component/FractureManageComponent.FractureManageComponent_C|GetESWCode (Variables|Default|GetFractureManageComponent)))
  (if (not (Variables|/Game/Prop/_Base_Component/FractureManageComponent.FractureManageComponent_C|GetisFractured (Variables|Default|GetFractureManageComponent)))
    ;[1 1 1] Change object state(ex cant be grabbed)
    (Default|SetCanGrab (Variables|Default|GetGrabManageComponent) false)
    (Variables|/Game/Prop/_Base_Component/FractureManageComponent.FractureManageComponent_C|SetisFractured (Variables|Default|GetFractureManageComponent) true)
    ;[1 1 1] GAME INSTANCE
    (bind _asbp_game_instance_2 (Utilities|Casting|CastToBP_GameInstance (Game|GetGameInstance)))
    (bind _ns (Default|GetNsfromENSCode _asbp_game_instance_2 (Variables|/Game/Prop/_Base_Component/FractureManageComponent.FractureManageComponent_C|GetENSCode (Variables|Default|GetFractureManageComponent))))
    (Default|SpawnNsatLocation _asbp_game_instance_2 _ns (.location BreakEvent))
    (Default|EventDestroy _asbp_game_instance_2)))

(event EventBeginPlay
  (bind _geometrycollection (Variables|Default|GetGeometryCollection))
  (EventDispatchers|BindEventtoOnChaosPhysicsCollision _geometrycollection (EventDispatchers|CreateEvent :!event Custom|ChaosCollisionEvent))
  (EventDispatchers|BindEventtoOnChaosBreakEvent _geometrycollection (EventDispatchers|CreateEvent :!event Custom|ChaosBreakEvent))
  (Default|SetGrabbedObjectMass (Variables|Default|GetGrabManageComponent) (Variables|Default|GetGC_Mass)))

(event Collision|EventActorBeginOverlap
  (params (OtherActor :type Actor%20Object%20Reference)))

(event EventTick
  (params (DeltaSeconds :type Float%20%28single-precision%29)))

(fn ConstructionScript)