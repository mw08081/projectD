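; BP_Donut4 is a grabbable, destructible donut prop that awards score when broken.
; Overlapping punch, delayed or bomb fields trigger sounds; sufficient strain or any bomb field converts it once to a random destroyed mesh with Niagara effects and score.
; When flagged, its next hit spawns a delayed field at the impact point, using strain derived from acceleration and mass to carry thrown-impact damage.
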(event OnComponentBeginOverlap(StaticMesh)
  (params (OverlappedComponent :type Primitive%20Component%20Object%20Reference) (OtherActor :type Actor%20Object%20Reference) (OtherComp :type Primitive%20Component%20Object%20Reference) (OtherBodyIndex :type Integer) (bFromSweep :type Boolean) (SweepResult :type Hit%20Result%20Structure%20%28by%20ref%29))
  (bind _bp_gameinstance (Variables|Default|GetBP_GameInstance))
  (bind _lvobjectroot (Variables|Default|GetLvObjectRoot))
  (bind _objectprice (Variables|/Script/ProjectD.LvObjectRoot|GetobjectPrice _lvobjectroot))
  ;[1 1 1] Triggered by Punch
  (bind _asbp_master_field (Utilities|Casting|CastToBP_MasterField OtherActor)
    (:then
      (if (and (Variables|/Game/_FiledSystem/BP_MasterField.BP_MasterField_C|GetField%20Active _asbp_master_field) (> (Variables|/Game/_FiledSystem/BP_MasterField.BP_MasterField_C|GetStrain%20Magnitude _asbp_master_field) (Variables|/Game/Prop/_Base/_Base_Component/ConvertManageComponent.ConvertManageComponent_C|GetDmgThreshold (Variables|Default|GetConvertManageComponent))))
        (Default|PlaySfx (Variables|Default|GetSfxPlayComponent) "NewEnumerator0" :!label _label)
        (if (not (Variables|/Game/Prop/_Base/_Base_Component/ConvertManageComponent.ConvertManageComponent_C|GetisConverted (Variables|Default|GetConvertManageComponent)))
          ;[1 1 1] GI
          (CallFunction|ChangeActorState)
          (bind _ns (Default|GetNsfromENSCode _bp_gameinstance (Variables|/Game/Prop/_Base/_Base_Component/ConvertManageComponent.ConvertManageComponent_C|GetEvent_ENSCode (Variables|Default|GetConvertManageComponent))))
          (Default|SpawnNsatLocation _bp_gameinstance _ns (Transformation|GetActorLocation))
          (bind _asproject_d_default_game_mode (Utilities|Casting|CastToProjectD_DefaultGameMode (Game|GetGameMode)))
          (Class|ProjectDDefaultGameMode|SpawnFloatingScore _asproject_d_default_game_mode (Transformation|GetActorLocation) _objectprice)
          (Utilities|FlowControl|Delay 1.0)
          (Class|ProjectDDefaultGameMode|GetScore _asproject_d_default_game_mode _objectprice))
        (else
          (Default|PlaySfx (Variables|Default|GetSfxPlayComponent) "NewEnumerator1" :!label _label_2))))
    (:CastFailed
      ;[1 1 1] Triggered by DMF
      (bind _asbp_delay_master_field (Utilities|Casting|CastToBP_DelayMasterField OtherActor)
        (:then
          (Default|SpawnHitNsatLocation (Variables|Default|GetBP_GameInstance) (Transformation|GetActorLocation))
          (if (> (Variables|/Game/_FiledSystem/BP_DelayMasterField.BP_DelayMasterField_C|GetStrain%20Magnitude _asbp_delay_master_field) (Variables|/Game/Prop/_Base/_Base_Component/ConvertManageComponent.ConvertManageComponent_C|GetDmgThreshold (Variables|Default|GetConvertManageComponent)))
            (goto _label)
            (else
              (goto _label_2))))
        (:CastFailed
          ;[1 1 1] Triggerd By Bomb
          (bind _asbp_bomb_field (Utilities|Casting|CastToBP_BombField OtherActor)
            (:then
              (if (Variables|/Game/_FiledSystem/BP_BombField.BP_BombField_C|GetuseBomb _asbp_bomb_field)
                (Class|PrimitiveComponent|WakeRigidBody (Variables|Default|GetStaticMesh) "None")
                (Default|SpawnHitNsatLocation (Variables|Default|GetBP_GameInstance) (Transformation|GetActorLocation))
                (goto _label)
                (else
                  (goto _label))))
            (:CastFailed
              (Development|PrintString "all cast failed"))))))))

(event OnComponentHit(StaticMesh)
  (params (HitComponent :type Primitive%20Component%20Object%20Reference) (OtherActor :type Actor%20Object%20Reference) (OtherComp :type Primitive%20Component%20Object%20Reference) (NormalImpulse :type Vector :default "0, 0, 0") (Hit :type Hit%20Result%20Structure%20%28by%20ref%29))
  (bind _impactpoint (Collision|BreakHitResult Hit))
  (Default|PlaySfx (Variables|Default|GetSfxPlayComponent) "NewEnumerator2")
  ;[1 1 1] Delay Master field when be thrown
  (if (Variables|Default|GetShouldSpawnDMF)
    (Variables|Default|SetShouldSpawnDMF false)
    (bind _returnvalue (Game|SpawnActorfromClass "/Game/_FiledSystem/BP_DelayMasterField.BP_DelayMasterField_C" (Math|Conversions|ToTransform(Vector) _impactpoint) "AlwaysSpawn" "MultiplyWithRoot" 0 0))
    (Default|InitDMF :self _returnvalue :ImpactPoint _impactpoint :StrainMagnitude (Variables|Default|GetTargetStrainMagnitude))))

(event EventBeginPlay
  (bind _staticmesh (Variables|Default|GetStaticMesh))
  (bind _grabmanagecomponent (Variables|Default|GetGrabManageComponent))
  (Default|SetGrabbedStaticMesh _grabmanagecomponent (Variables|/Script/Engine.StaticMeshComponent|GetStaticMesh _staticmesh))
  (Default|SetGrabbedObjectMass _grabmanagecomponent (Physics|GetMass _staticmesh))
  (bind _asbp_game_instance (Utilities|Casting|CastToBP_GameInstance (Game|GetGameInstance)))
  (Variables|Default|SetBP_GameInstance _asbp_game_instance))

(event Collision|EventActorBeginOverlap
  (params (OtherActor :type Actor%20Object%20Reference)))

(event EventTick
  (params (DeltaSeconds :type Float%20%28single-precision%29)))

(fn ConstructionScript)

(fn ChangeActorState
  (bind _convertmanagecomponent (Variables|Default|GetConvertManageComponent))
  (bind _staticmesh (Variables|Default|GetStaticMesh))
  (bind _destroyed_target_staticmesh (Variables|/Game/Prop/_Base/_Base_Component/ConvertManageComponent.ConvertManageComponent_C|GetDESTROYED_TARGET_STATICMESH _convertmanagecomponent))
  (bind _outitem (Utilities|Array|Random _destroyed_target_staticmesh))
  ;[1 1 1] Change State
  (Variables|/Game/Prop/_Base/_Base_Component/ConvertManageComponent.ConvertManageComponent_C|SetisConverted (Variables|Default|GetConvertManageComponent) true)
  (if (> (Utilities|Array|Length _destroyed_target_staticmesh) 0)
    (Components|StaticMesh|SetStaticMesh _staticmesh _outitem)
    (Rendering|Material|SetMaterial _staticmesh 0 (Variables|/Game/Prop/_Base/_Base_Component/ConvertManageComponent.ConvertManageComponent_C|GetDESTROYED_TARGET_MATERIAL _convertmanagecomponent))
    (Default|SetGrabbedStaticMesh (Variables|Default|GetGrabManageComponent) _outitem)))

(fn SetTargetStrainMagnitude
  (params (_ACC :type Float%20%28double-precision%29))
  (Variables|Default|SetTargetStrainMagnitude (* _ACC 1e+03 (Physics|GetMass (Variables|Default|GetStaticMesh)))))