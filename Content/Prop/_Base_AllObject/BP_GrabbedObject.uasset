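; BP_GrabbedObject is the stand-in for a grabbed, thrown prop that turns back into its original actor's class on first impact.
; SetGrabData stores the original actor and field activation type, while SetFractureData stores the throw transform and scales magnitude from charge time.
; The first hit spawns a BP_DelayMasterField, using throw rotation and directional force only on upward-facing surfaces.
; It then spawns the original class there and destroys itself.
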(event OnComponentHit(StaticMesh)
  (params (HitComponent :type Primitive%20Component%20Object%20Reference) (OtherActor :type Actor%20Object%20Reference) (OtherComp :type Primitive%20Component%20Object%20Reference) (NormalImpulse :type Vector :default "0, 0, 0") (Hit :type Hit%20Result%20Structure%20%28by%20ref%29))
  (if (not (Variables|SpawnData|GetisSpawnOrgActor))
    (Rendering|Debug|DrawDebugSphere (.impactpoint Hit) 1e+01 12 "(R=0.612927,G=0.000000,B=1.000000,A=1.000000)" 5.0)
    (Variables|SpawnData|SetisSpawnOrgActor true)
    (Collision|SetCollisionProfileName (Variables|Default|GetStaticMesh) "NoCollision" true :!class /Script/Engine.PrimitiveComponent)
    (Utilities|FlowControl|Delay 0.001)
    (bind _shouldapplydirectionalmagnitude (CallFunction|GetSholdCalcDirectionalMagnitude (.normal Hit)))
    (if _shouldapplydirectionalmagnitude
      (bind _directionalmagnitudetransform (CallFunction|GetDirectionalMagnitudeTransform (.impactpoint Hit)))
      (Variables|SpawnData|SetDelayMsFsTransform _directionalmagnitudetransform)
      (else
        (Variables|SpawnData|SetDelayMsFsTransform (Math|Conversions|ToTransform(Vector) (.impactpoint Hit)))))
    (bind _returnvalue (Game|SpawnActorfromClass "/Game/Prop/_FiledSystem/BP_DelayMasterField.BP_DelayMasterField_C" (Variables|SpawnData|GetDelayMsFsTransform) "Undefined" "MultiplyWithRoot" 0 0))
    (Variables|/Game/Prop/_FiledSystem/BP_DelayMasterField.BP_DelayMasterField_C|SetUseDirectionalVector _returnvalue _shouldapplydirectionalmagnitude)
    (Variables|/Game/Prop/_FiledSystem/BP_DelayMasterField.BP_DelayMasterField_C|SetDirectionalMagnitude _returnvalue (Variables|FractureData|GetDelayMsFs_DirectionalMagnitude))
    (Variables|/Game/Prop/_FiledSystem/BP_DelayMasterField.BP_DelayMasterField_C|SetActivationType _returnvalue (Variables|GrabData|GetEField_ActiavationType))
    (Game|SpawnActorfromClass (Utilities|GetClass (Variables|GrabData|GetOrgActor)) (Math|Conversions|ToTransform(Vector) (.impactpoint Hit)) "AlwaysSpawn" "MultiplyWithRoot" 0 0)
    (Actor|DestroyActor)))

(event EventBeginPlay)

(event Collision|EventActorBeginOverlap
  (params (OtherActor :type Actor%20Object%20Reference)))

(event EventTick
  (params (DeltaSeconds :type Float%20%28single-precision%29)))

(fn ConstructionScript)

(fn GetSholdCalcDirectionalMagnitude
  (params (HitNormal :type Vector))
  (if (> (.z HitNormal) 0.75)
    (return true)
    (else
      (return false))))

(fn GetDirectionalMagnitudeTransform
  (params (ImpactPoint :type Vector))
  (return (Math|Transform|MakeTransform ImpactPoint (.rotation (Variables|FractureData|GetThrowingTransform)))))

(fn SetFractureData
  (params (ThrowingTransform :type Transform) (ElapsedChargeTime :type Float%20%28double-precision%29))
  (Variables|FractureData|SetThrowingTransform ThrowingTransform)
  (Variables|FractureData|SetDelayMsFs_DirectionalMagnitude (+ (* (* ElapsedChargeTime 0.5) (- (Variables|FractureData|Constant|GetMAX_DELAY_MS_FS_DIRECTIONAL_MAGNITUDE) (Variables|FractureData|Constant|GetMIN_DELAY_MS_FS_DIRECTIONAL_MAGNITUDE))) (Variables|FractureData|Constant|GetMIN_DELAY_MS_FS_DIRECTIONAL_MAGNITUDE))))

(fn SetGrabData
  (params (OrgActor :type Actor%20Object%20Reference) (EField_ActivationType :type EFieldActivationType%20Enum :default "NewEnumerator0"))
  (Variables|GrabData|SetOrgActor OrgActor)
  (Variables|GrabData|SetEField_ActiavationType EField_ActivationType))