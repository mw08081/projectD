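; BP_NsObject is a prop actor that plays a short burst of a Niagara effect supplied by the caller.
; SetNs assigns the effect to the Niagara component, resetting existing override parameters, and raises the CanPlay flag.
; Tick polls that flag, clears it, activates the component, then deactivates it after a brief delay.
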(event EventBeginPlay)

(event Collision|EventActorBeginOverlap
  (params (OtherActor :type Actor%20Object%20Reference)))

(event EventTick
  (params (DeltaSeconds :type Float%20%28single-precision%29))
  (if (Variables|Default|GetcanPlay)
    (Variables|Default|SetcanPlay false)
    (Components|Activation|Activate (Variables|Default|GetNiagara) false)
    (Utilities|FlowControl|Delay 0.2)
    (Components|Activation|Deactivate (Variables|Default|GetNiagara))))

(fn ConstructionScript)

(fn SetNs
  (params (E_NsCode :type Niagara%20System%20Object%20Reference))
  (Class|NiagaraComponent|SetAsset (Variables|Default|GetNiagara) E_NsCode true)
  (Variables|Default|SetcanPlay true))