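; Base prop that vanishes outright when struck by a strong enough field, passing its mesh and mass to GrabManageComponent on BeginPlay.
; Overlaps with BP_MasterField or BP_DelayMasterField compare StrainMagnitude against DmgThreshold, while the hit check always returns false here.
; On success it spawns a BP_NsObject with the FractureManageComponent's Niagara effect if unfractured, triggers sound and EventDestroy through BP_GameInstance, then destroys itself.
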(event OnComponentHit(StaticMesh)
  (params (HitComponent :type Primitive%20Component%20Object%20Reference) (OtherActor :type Actor%20Object%20Reference) (OtherComp :type Primitive%20Component%20Object%20Reference) (NormalImpulse :type Vector :default "0, 0, 0") (Hit :type Hit%20Result%20Structure%20%28by%20ref%29))
  ;[1 1 1] Dont need to Set/Get Is Fractured. Because it will be disappear perfactly
  (bind _shoulddisappear (CallFunction|CheckDisappearConditionbyHit Hit))
  (if _shoulddisappear
    (CallFunction|PlayEventDisappearNs)
    (CallFunction|PlayEventDisappearSound)
    (Actor|DestroyActor)))

(event OnComponentBeginOverlap(StaticMesh)
  (params (OverlappedComponent :type Primitive%20Component%20Object%20Reference) (OtherActor :type Actor%20Object%20Reference) (OtherComp :type Primitive%20Component%20Object%20Reference) (OtherBodyIndex :type Integer) (bFromSweep :type Boolean) (SweepResult :type Hit%20Result%20Structure%20%28by%20ref%29))
  ;[1 1 1] Dont need to Set/Get Is Fractured. Because it will be disappear perfactly
  (bind _shoulddisappear (CallFunction|CheckDisappearConditionbyOverlap OtherActor SweepResult))
  (if _shoulddisappear
    (CallFunction|PlayEventDisappearNs)
    (CallFunction|PlayEventDisappearSound)
    (Actor|DestroyActor)))

(event EventBeginPlay
  (bind _staticmesh (Variables|Default|GetStaticMesh))
  (bind _grabmanagecomponent (Variables|Default|GetGrabManageComponent))
  (Default|SetGrabbedStaticMesh _grabmanagecomponent (Variables|/Script/Engine.StaticMeshComponent|GetStaticMesh _staticmesh))
  (Default|SetGrabbedObjectMass _grabmanagecomponent (Physics|GetMass _staticmesh)))

(event Collision|EventActorBeginOverlap
  (params (OtherActor :type Actor%20Object%20Reference)))

(event EventTick
  (params (DeltaSeconds :type Float%20%28single-precision%29)))

(fn ConstructionScript)

(fn CheckDisappearConditionbyOverlap
  (params (OtherActor :type Actor%20Object%20Reference) (SweepResult :type Hit%20Result%20Structure))
  (bind _dmgthreshold (Variables|Default|GetDmgThreshold))
  (bind _asbp_master_field (Utilities|Casting|CastToBP_MasterField OtherActor)
    (:then
      (Development|PrintString (Utilities|String|ToString(Float) (Variables|/Game/Prop/_FiledSystem/BP_MasterField.BP_MasterField_C|GetStrain%20Magnitude _asbp_master_field)))
      (return (> (Variables|/Game/Prop/_FiledSystem/BP_MasterField.BP_MasterField_C|GetStrain%20Magnitude _asbp_master_field) _dmgthreshold)))
    (:CastFailed
      (bind _asbp_delay_master_field (Utilities|Casting|CastToBP_DelayMasterField OtherActor)
        (:then
          (Development|PrintString (Utilities|String|ToString(Float) (Variables|/Game/Prop/_FiledSystem/BP_DelayMasterField.BP_DelayMasterField_C|GetStrain%20Magnitude _asbp_delay_master_field)))
          (return (> (Variables|/Game/Prop/_FiledSystem/BP_DelayMasterField.BP_DelayMasterField_C|GetStrain%20Magnitude _asbp_delay_master_field) _dmgthreshold)))
        (:CastFailed
          (Development|PrintString "All cast failed"))))))

(fn CheckDisappearConditionbyHit
  (params (HitResult :type Hit%20Result%20Structure))
  (return false))

(fn PlayEventDisappearSound
  (bind _asbp_game_instance (Utilities|Casting|CastToBP_GameInstance (Game|GetGameInstance)))
  (Default|SpawnSoundatLocation _asbp_game_instance "0, 0, 0" (Variables|/Game/Prop/_Base_Component/FractureManageComponent.FractureManageComponent_C|GetESWCode (Variables|Default|GetFractureManageComponent)))
  (Default|EventDestroy _asbp_game_instance))

(fn PlayEventDisappearNs
  (bind _fracturemanagecomponent (Variables|Default|GetFractureManageComponent))
  (if (not (Variables|/Game/Prop/_Base_Component/FractureManageComponent.FractureManageComponent_C|GetisFractured _fracturemanagecomponent))
    (bind _returnvalue (Game|SpawnActorfromClass "/Game/Prop/_ActionObject/BP_NsObject.BP_NsObject_C" (Transformation|GetActorTransform) "Undefined" "MultiplyWithRoot" 0 0))
    (bind _fracturingns (Default|GetFracturingNs _fracturemanagecomponent))
    (Default|SetNs _returnvalue _fracturingns)))