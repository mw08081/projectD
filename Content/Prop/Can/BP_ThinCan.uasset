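; BP_ThinCan is a thin can prop that plays a collision sound once it has been converted.
; Static mesh hits check ConvertManageComponent's IsConverted flag, then pass the SoundComponent's ESW code to BP_GameInstance to spawn a sound at the can's location.
; The PlayAfterConvertingCollisionSound override calls its parent, then spawns the same sound without checking the flag.
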(event OnComponentHit(StaticMesh)
  (params (HitComponent :type Primitive%20Component%20Object%20Reference) (OtherActor :type Actor%20Object%20Reference) (OtherComp :type Primitive%20Component%20Object%20Reference) (NormalImpulse :type Vector :default "0, 0, 0") (Hit :type Hit%20Result%20Structure%20%28by%20ref%29))
  (if (Variables|/Game/Prop/_Base_Component/ConvertManageComponent.ConvertManageComponent_C|GetisConverted (Variables|Default|GetConvertManageComponent))
    (bind _eswcode (Default|GetESWCode (Variables|Default|GetSoundComponent)))
    (bind _asbp_game_instance (Utilities|Casting|CastToBP_GameInstance (Game|GetGameInstance)))
    (Default|SpawnSoundatLocation _asbp_game_instance (Transformation|GetActorLocation) _eswcode)))

(event EventBeginPlay
  (|CallParentFunction) ; This node is disabled and will not be called.\nDrag off pins to build functionality.
)

(event Collision|EventActorBeginOverlap
  (params (OtherActor :type Actor%20Object%20Reference))
  (|CallParentFunction OtherActor) ; This node is disabled and will not be called.\nDrag off pins to build functionality.
)

(event EventTick
  (params (DeltaSeconds :type Float%20%28single-precision%29))
  (|CallParentFunction DeltaSeconds) ; This node is disabled and will not be called.\nDrag off pins to build functionality.
)

(fn ConstructionScript
  (|CallParentFunction))

(fn PlayAfterConvertingCollisionSound
  (|CallParentFunction)
  (bind _eswcode (Default|GetESWCode (Variables|Default|GetSoundComponent)))
  (bind _asbp_game_instance (Utilities|Casting|CastToBP_GameInstance (Game|GetGameInstance)))
  (Default|SpawnSoundatLocation _asbp_game_instance (Transformation|GetActorLocation) _eswcode))