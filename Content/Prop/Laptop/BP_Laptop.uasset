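; Breakable laptop prop with an upper static mesh and a Geometry Collection base that shatters when struck or thrown.
; Overlaps with FS_MasterField-tagged components compare the master or delay field's strain against damage thresholds.
; A break disables the box collider, simulates the base (detached first for delay fields), then spawns the FractureManageComponent's effect and sound.
; Physics hit events are left unwired, so only field overlaps trigger breaking.
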(event OnComponentHit(SM_Laptop_upper)
  (params (HitComponent :type Primitive%20Component%20Object%20Reference) (OtherActor :type Actor%20Object%20Reference) (OtherComp :type Primitive%20Component%20Object%20Reference) (NormalImpulse :type Vector :default "0, 0, 0") (Hit :type Hit%20Result%20Structure%20%28by%20ref%29))
  ;[1 1 1] laptop gc가 직접적으로 충돌할 일이 없어졌습니다.
)

(event OnComponentHit(GC_Laptop_under_boxCollider)
  (params (HitComponent :type Primitive%20Component%20Object%20Reference) (OtherActor :type Actor%20Object%20Reference) (OtherComp :type Primitive%20Component%20Object%20Reference) (NormalImpulse :type Vector :default "0, 0, 0") (Hit :type Hit%20Result%20Structure%20%28by%20ref%29))
  ;[1 1 1] laptop gc가 직접적으로 충돌할 일이 없어졌습니다.
)

(event OnComponentBeginOverlap(SM_Laptop_upper)
  (params (OverlappedComponent :type Primitive%20Component%20Object%20Reference) (OtherActor :type Actor%20Object%20Reference) (OtherComp :type Primitive%20Component%20Object%20Reference) (OtherBodyIndex :type Integer) (bFromSweep :type Boolean) (SweepResult :type Hit%20Result%20Structure%20%28by%20ref%29))
  (bind _returnvalue (Components|GetOwner OtherComp))
  (bind _gc_laptop_under (Variables|Default|GetGC_Laptop_under))
  (if (Components|ComponentHasTag OtherComp "FS_MasterField")
    (bind _asbp_master_field (Utilities|Casting|CastToBP_MasterField _returnvalue)
      (:then
        (if (> (Variables|/Game/Prop/_FiledSystem/BP_MasterField.BP_MasterField_C|GetStrain%20Magnitude _asbp_master_field) (Variables|Default|GetHitDamamgeThreshold))
          (Collision|SetCollisionProfileName (Variables|Default|GetGC_Laptop_under_boxCollider) "NoCollision" true :!class /Script/Engine.PrimitiveComponent)
          (Physics|SetSimulatePhysics (Variables|Default|GetGC_Laptop_under) true)
          (CallFunction|FractureLaptopUpper)
          (Development|PrintString "over break")))
      (:CastFailed
        (bind _asbp_delay_master_field (Utilities|Casting|CastToBP_DelayMasterField _returnvalue))
        (if (> (Variables|/Game/Prop/_FiledSystem/BP_DelayMasterField.BP_DelayMasterField_C|GetStrain%20Magnitude _asbp_delay_master_field) (Variables|Default|GetCollisionDamageThreshold))
          (Transformation|DetachFromComponent _gc_laptop_under "KeepWorld" "KeepWorld" "KeepWorld" true)
          (Physics|SetSimulatePhysics _gc_laptop_under true)
          (Collision|SetCollisionProfileName (Variables|Default|GetGC_Laptop_under_boxCollider) "NoCollision" true :!class /Script/Engine.PrimitiveComponent)
          (CallFunction|FractureLaptopUpper)
          (Development|PrintString "throwing break"))))))

(event OnComponentBeginOverlap(GC_Laptop_under)
  (params (OverlappedComponent :type Primitive%20Component%20Object%20Reference) (OtherActor :type Actor%20Object%20Reference) (OtherComp :type Primitive%20Component%20Object%20Reference) (OtherBodyIndex :type Integer) (bFromSweep :type Boolean) (SweepResult :type Hit%20Result%20Structure%20%28by%20ref%29))
  (if (Components|ComponentHasTag OtherComp "FS_MasterField")
    (bind _asbp_master_field (Utilities|Casting|CastToBP_MasterField (Components|GetOwner OtherComp)))
    (if (> (Variables|/Game/Prop/_FiledSystem/BP_MasterField.BP_MasterField_C|GetStrain%20Magnitude _asbp_master_field) (Variables|Default|GetHitDamamgeThreshold))
      (Collision|SetCollisionProfileName (Variables|Default|GetGC_Laptop_under_boxCollider) "NoCollision" true :!class /Script/Engine.PrimitiveComponent)
      (Physics|SetSimulatePhysics (Variables|Default|GetGC_Laptop_under) true)
      (CallFunction|FractureLaptopUpper)
      (Development|PrintString "over break"))))

(event EventBeginPlay)

(event Collision|EventActorBeginOverlap
  (params (OtherActor :type Actor%20Object%20Reference)))

(event EventTick
  (params (DeltaSeconds :type Float%20%28single-precision%29)))

(fn ConstructionScript)

(fn FractureLaptopUpper
  (bind _returnvalue (Transformation|GetActorLocation))
  (bind _fracturemanagecomponent (Variables|Default|GetFractureManageComponent))
  (bind _returnvalue_2 (Game|SpawnActorfromClass "/Game/Prop/_Base_AllObject/BP_NsObject.BP_NsObject_C" (Math|Conversions|ToTransform(Vector) _returnvalue) "AdjustIfPossibleButAlwaysSpawn" "MultiplyWithRoot" 0 0))
  (bind _fracturingns (Default|GetFracturingNs _fracturemanagecomponent))
  (Default|SetNs _returnvalue_2 _fracturingns)
  (bind _asbp_game_instance (Utilities|Casting|CastToBP_GameInstance (Game|GetGameInstance)))
  (Default|SpawnSoundatLocation _asbp_game_instance _returnvalue (Variables|/Game/Prop/_Base_FractureObject/FractureManageComponent.FractureManageComponent_C|GetESWCode _fracturemanagecomponent)))