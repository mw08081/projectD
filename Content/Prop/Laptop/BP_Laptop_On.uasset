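; Breakable, grabbable laptop prop that shatters when a sufficiently strong field actor overlaps it.
; Upper mesh and lower box overlaps compare master field strain to a damage threshold; only the upper also accepts delay fields.
; Breaking detaches the lower Geometry Collection into physics, disables grabbing, and swaps the upper mesh to a destroyed material.
; GameInstance spawns the Niagara effect and sound from FractureManageComponent codes, then receives a destroy event.
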(event OnComponentHit(SM_Laptop_upper)
  (params (HitComponent :type Primitive%20Component%20Object%20Reference) (OtherActor :type Actor%20Object%20Reference) (OtherComp :type Primitive%20Component%20Object%20Reference) (NormalImpulse :type Vector :default "0, 0, 0") (Hit :type Hit%20Result%20Structure%20%28by%20ref%29))
  ;[1 1 1] laptop gc가 직접적으로 충돌할 일이 없어졌습니다.
)

(event OnComponentHit(GC_Laptop_under_boxCollider)
  (params (HitComponent :type Primitive%20Component%20Object%20Reference) (OtherActor :type Actor%20Object%20Reference) (OtherComp :type Primitive%20Component%20Object%20Reference) (NormalImpulse :type Vector :default "0, 0, 0") (Hit :type Hit%20Result%20Structure%20%28by%20ref%29))
  ;[1 1 1] laptop gc가 직접적으로 충돌할 일이 없어졌습니다.
)

(event OnComponentBeginOverlap(GC_Laptop_under_boxCollider)
  (params (OverlappedComponent :type Primitive%20Component%20Object%20Reference) (OtherActor :type Actor%20Object%20Reference) (OtherComp :type Primitive%20Component%20Object%20Reference) (OtherBodyIndex :type Integer) (bFromSweep :type Boolean) (SweepResult :type Hit%20Result%20Structure%20%28by%20ref%29))
  (bind _gc_laptop_under (Variables|Default|GetGC_Laptop_under))
  (if (and (Components|ComponentHasTag OtherComp "FS_MasterField") (not (Variables|/Game/Prop/_Base_Component/FractureManageComponent.FractureManageComponent_C|GetisFractured (Variables|Default|GetFractureManageComponent))))
    (bind _asbp_master_field (Utilities|Casting|CastToBP_MasterField (Components|GetOwner OtherComp)))
    (if (> (Variables|/Game/Prop/_FiledSystem/BP_MasterField.BP_MasterField_C|GetStrain%20Magnitude _asbp_master_field) (Variables|Default|GetHitDamamgeThreshold))
      (Collision|SetCollisionProfileName (Variables|Default|GetGC_Laptop_under_boxCollider) "NoCollision" true :!class /Script/Engine.PrimitiveComponent)
      (Transformation|DetachFromComponent _gc_laptop_under "KeepWorld" "KeepWorld" "KeepWorld" true)
      (Physics|SetSimulatePhysics _gc_laptop_under true)
      (CallFunction|FractureLaptopUpper)
      (Default|SetCanGrab (Variables|Default|GetGrabManageComponent) false)
      (Variables|/Game/Prop/_Base_Component/FractureManageComponent.FractureManageComponent_C|SetisFractured (Variables|Default|GetFractureManageComponent) true))))

(event OnComponentBeginOverlap(SM_Laptop_upper)
  (params (OverlappedComponent :type Primitive%20Component%20Object%20Reference) (OtherActor :type Actor%20Object%20Reference) (OtherComp :type Primitive%20Component%20Object%20Reference) (OtherBodyIndex :type Integer) (bFromSweep :type Boolean) (SweepResult :type Hit%20Result%20Structure%20%28by%20ref%29))
  (bind _returnvalue (Components|GetOwner OtherComp))
  (bind _gc_laptop_under (Variables|Default|GetGC_Laptop_under))
  (if (and (Components|ComponentHasTag OtherComp "FS_MasterField") (not (Variables|/Game/Prop/_Base_Component/FractureManageComponent.FractureManageComponent_C|GetisFractured (Variables|Default|GetFractureManageComponent))))
    (bind _asbp_master_field (Utilities|Casting|CastToBP_MasterField _returnvalue)
      (:then
        (if (> (Variables|/Game/Prop/_FiledSystem/BP_MasterField.BP_MasterField_C|GetStrain%20Magnitude _asbp_master_field) (Variables|Default|GetHitDamamgeThreshold))
          (Collision|SetCollisionProfileName (Variables|Default|GetGC_Laptop_under_boxCollider) "NoCollision" true :!class /Script/Engine.PrimitiveComponent :!label _label)
          (Transformation|DetachFromComponent _gc_laptop_under "KeepWorld" "KeepWorld" "KeepWorld" true)
          (Physics|SetSimulatePhysics _gc_laptop_under true)
          (CallFunction|FractureLaptopUpper)
          (Default|SetCanGrab (Variables|Default|GetGrabManageComponent) false)
          (Variables|/Game/Prop/_Base_Component/FractureManageComponent.FractureManageComponent_C|SetisFractured (Variables|Default|GetFractureManageComponent) true)))
      (:CastFailed
        (bind _asbp_delay_master_field (Utilities|Casting|CastToBP_DelayMasterField _returnvalue))
        (if (> (Variables|/Game/Prop/_FiledSystem/BP_DelayMasterField.BP_DelayMasterField_C|GetStrain%20Magnitude _asbp_delay_master_field) (Variables|Default|GetHitDamamgeThreshold))
          (goto _label))))))

(event EventBeginPlay
  (Default|SetGrabbedObjectMass (Variables|Default|GetGrabManageComponent) (Physics|GetMass (Variables|Default|GetSM_Laptop_upper))))

(event Collision|EventActorBeginOverlap
  (params (OtherActor :type Actor%20Object%20Reference)))

(event EventTick
  (params (DeltaSeconds :type Float%20%28single-precision%29)))

(fn ConstructionScript)

(fn FractureLaptopUpper
  (bind _returnvalue (Transformation|GetActorLocation))
  (bind _fracturemanagecomponent (Variables|Default|GetFractureManageComponent))
  (Rendering|Material|SetMaterial (Variables|Default|GetSM_Laptop_upper) 0 "/Game/Prop/Laptop/Texture/d_texture/M_LaptopDestroyed.M_LaptopDestroyed")
  (bind _asbp_game_instance (Utilities|Casting|CastToBP_GameInstance (Game|GetGameInstance)))
  (bind _ns (Default|GetNsfromENSCode _asbp_game_instance (Variables|/Game/Prop/_Base_Component/FractureManageComponent.FractureManageComponent_C|GetENSCode _fracturemanagecomponent)))
  (Default|SpawnNsatLocation _asbp_game_instance _ns _returnvalue)
  (Default|SpawnSoundatLocation _asbp_game_instance _returnvalue (Variables|/Game/Prop/_Base_Component/FractureManageComponent.FractureManageComponent_C|GetESWCode _fracturemanagecomponent))
  (Default|EventDestroy _asbp_game_instance))