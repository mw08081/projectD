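; Stand-in prop for a grabbed object that gets thrown, storing the original actor and mass plus the throw transform and charge time.
; On the first hit with CanSpawnOrgActor set, it spawns a BP_DelayMasterField using impact point, charge- and mass-scaled strain, and charge-based directional magnitude.
; It then destroys itself, spawns a fresh instance of the original's class in place and plays a pooled Ns effect.
; Falling-detection debug logic is unconnected.
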(event OnComponentHit(StaticMesh)
  (params (HitComponent :type Primitive%20Component%20Object%20Reference) (OtherActor :type Actor%20Object%20Reference) (OtherComp :type Primitive%20Component%20Object%20Reference) (NormalImpulse :type Vector :default "0, 0, 0") (Hit :type Hit%20Result%20Structure%20%28by%20ref%29))
  (bind _returnvalue (Transformation|GetActorTransform))
  (if (Variables|Default|GetcanSpawnOrgActor)
    (if (not (Variables|SpawnData|GetisSpawnOrgActor))
      (Variables|SpawnData|SetisSpawnOrgActor true)
      (Collision|SetCollisionProfileName (Variables|Default|GetStaticMesh) "NoCollision" true :!class /Script/Engine.PrimitiveComponent)
      (Utilities|FlowControl|Delay 0.0)
      (bind _returnvalue_2 (Game|SpawnActorfromClass "/Game/_FiledSystem/BP_DelayMasterField.BP_DelayMasterField_C" (Math|Transform|MakeTransform "0, 0, 0") "AdjustIfPossibleButAlwaysSpawn" "OverrideRootScale" 0 0))
      (Default|InitDMF _returnvalue_2 (Variables|FractureData|GetThrowingTransform) (.impactpoint Hit) (* (Math|Float|Clamp(Float) (* (Variables|FractureData|GetelapsedChargeTime) 1e+01) 1.0 1e+01) (Variables|GrabData|GetGrabbedObjectMass) 1e+03) (Variables|FractureData|GetDelayMsFs_DirectionalMagnitude))
      (Actor|DestroyActor)
      (Game|SpawnActorfromClass (Utilities|GetClass (Variables|GrabData|GetOrgActor)) (Math|Transform|MakeTransform (.location _returnvalue) (.rotation _returnvalue) (.scale _returnvalue)) "AlwaysSpawn" "OverrideRootScale" 0 0)
      (bind _asbp_game_instance (Utilities|Casting|CastToBP_GameInstance (Game|GetGameInstance)))
      (bind _ns (Default|GetNsfromENSCode _asbp_game_instance "NewEnumerator0"))
      (bind _asbp_project_d_default_game_mode (Utilities|Casting|CastToBP_ProjectD_DefaultGameMode (Game|GetGameMode)))
      (bind _returnvalue_3 (Class|ObjectPoolSystem|GetPooledObjectNsDisplay (Variables|/Script/ProjectD.ProjectD_DefaultGameMode|GetObjectPool _asbp_project_d_default_game_mode)))
      (Transformation|SetActorLocation _returnvalue_3 (Transformation|GetActorLocation) false false)
      (Class|NsDisplay|SetNs _returnvalue_3 _ns))))

(event Custom|Falling)

(event EventBeginPlay)

(event Collision|EventActorBeginOverlap
  (params (OtherActor :type Actor%20Object%20Reference)))

(event EventTick
  (params (DeltaSeconds :type Float%20%28single-precision%29)))

(fn ConstructionScript)

(fn GetSholdCalcDirectionalMagnitude
  (params (HitNormal :type Vector))
  (if (> (.z HitNormal) 0.75)
    (return true)
    (else
      (return false))))

(fn GetDirectionalMagnitudeTransform
  (params (ImpactPoint :type Vector))
  (return (Math|Transform|MakeTransform ImpactPoint (.rotation (Variables|FractureData|GetThrowingTransform)) "0.350000,0.350000,0.350000")))

(fn SetThrowingData
  (params (ThrowingTransform :type Transform) (ElapsedChargeTime :type Float%20%28double-precision%29))
  (Variables|FractureData|SetThrowingTransform ThrowingTransform)
  (bind _output_get (Variables|FractureData|SetelapsedChargeTime ElapsedChargeTime))
  (Variables|FractureData|SetDelayMsFs_DirectionalMagnitude (+ (* _output_get (- (Variables|FractureData|Constant|GetMAX_DELAY_MS_FS_DIRECTIONAL_MAGNITUDE) (Variables|FractureData|Constant|GetMIN_DELAY_MS_FS_DIRECTIONAL_MAGNITUDE))) (Variables|FractureData|Constant|GetMIN_DELAY_MS_FS_DIRECTIONAL_MAGNITUDE))))

(fn SetGrabData
  (params (OrgActor :type Actor%20Object%20Reference) (OrgActorMass :type Float%20%28double-precision%29))
  (Variables|GrabData|SetOrgActor OrgActor)
  (Variables|GrabData|SetGrabbedObjectMass OrgActorMass))