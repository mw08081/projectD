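; BP_CombinedActor is a deprecated prop that groups two child actors and relays damage taken by the parent to both.
; On BeginPlay it makes itself the owner of both children, and its damage event logs the hit, then calls a custom ApplyDamage on each.
; That function checks LvObjectRoot's ObjectType: fracturing objects get a huge external strain on their BP_FractureObject geometry collection, ignoring damage amount, while others receive standard damage.
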(event Custom|OnTakeAnyDamage_Event
  (params (DamagedActor :type Actor%20Object%20Reference) (Damage :type Float%20%28single-precision%29) (DamageType :type Damage%20Type%20Object%20Reference) (InstigatedBy :type Controller%20Object%20Reference) (DamageCauser :type Actor%20Object%20Reference))
  (Development|PrintString (Utilities|String|Append (Utilities|GetDisplayName DamagedActor) "가 피격됨(" "(" (Utilities|GetDisplayName DamageCauser) "의한 데미지:" (Utilities|String|ToString(Float) Damage) ")"))
  (CallFunction|ApplyDamage (Variables|/Script/Engine.ChildActorComponent|GetChildActor (Variables|Default|GetChildActorComponent)) Damage InstigatedBy DamageCauser)
  (CallFunction|ApplyDamage (Variables|/Script/Engine.ChildActorComponent|GetChildActor (Variables|Default|GetChildActorComponent2)) Damage InstigatedBy DamageCauser))

(event EventBeginPlay
  (bind _self self)
  (Actor|SetOwner (Variables|/Script/Engine.ChildActorComponent|GetChildActor (Variables|Default|GetChildActorComponent)) _self)
  (Actor|SetOwner (Variables|/Script/Engine.ChildActorComponent|GetChildActor (Variables|Default|GetChildActorComponent2)) _self))

(event Collision|EventActorBeginOverlap
  (params (OtherActor :type Actor%20Object%20Reference)))

(event EventTick
  (params (DeltaSeconds :type Float%20%28single-precision%29)))

(fn ConstructionScript)

(fn ApplyDamage
  (params (DamagedActor :type Actor%20Object%20Reference) (Damage :type Float%20%28double-precision%29) (Instigator :type Controller%20Object%20Reference) (Casuer :type Actor%20Object%20Reference))
  (Development|PrintString (Utilities|GetDisplayName DamagedActor))
  (if (Utilities|Enum|Equal(Enum) (Variables|/Script/ProjectD.LvObjectRoot|GetobjectType (Actor|GetComponentbyClass DamagedActor "/Script/ProjectD.LvObjectRoot")) "FracturingObject")
    (bind _asbp_fracture_object (Utilities|Casting|CastToBP_FractureObject DamagedActor))
    (Class|GeometryCollectionComponent|ApplyExternalStrain (Variables|/Game/Prop/_Base/BP_FractureObject.BP_FractureObject_C|GetGeometryCollection _asbp_fracture_object) 0 (Transformation|GetActorLocation _asbp_fracture_object) 1e+02 0 1.0 111111111111.0)
    (else
      (Game|Damage|ApplyDamage DamagedActor Damage Instigator Casuer "/Script/Engine.DamageType"))))