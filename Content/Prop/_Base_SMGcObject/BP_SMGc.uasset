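; BP_SMGc is a base destructible prop that releases its GC component into physics when hit by a strong enough master field.
; Overlaps on its SM or GC components check for the FS_MasterField tag, then compare the owning BP_MasterField's StrainMagnitude against DamageThreshold.
; Above the threshold, both paths share one break sequence: detach GC in world space, enable physics simulation and turn off GCCollider's collision.
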(event OnComponentBeginOverlap(SM_)
  (params (OverlappedComponent :type Primitive%20Component%20Object%20Reference) (OtherActor :type Actor%20Object%20Reference) (OtherComp :type Primitive%20Component%20Object%20Reference) (OtherBodyIndex :type Integer) (bFromSweep :type Boolean) (SweepResult :type Hit%20Result%20Structure%20%28by%20ref%29))
  (bind _gc_ (Variables|Default|GetGC_))
  (if (Components|ComponentHasTag OtherComp "FS_MasterField")
    (bind _asbp_master_field (Utilities|Casting|CastToBP_MasterField (Components|GetOwner OtherComp)))
    (if (> (Variables|/Game/Prop/_FiledSystem/BP_MasterField.BP_MasterField_C|GetStrain%20Magnitude _asbp_master_field) (Variables|Default|GetDamageThreshold))
      (Transformation|DetachFromComponent _gc_ "KeepWorld" "KeepWorld" "KeepWorld" true)
      (Physics|SetSimulatePhysics _gc_ true)
      (Collision|SetCollisionProfileName (Variables|Default|GetGC_Collider) "NoCollision" true :!class /Script/Engine.PrimitiveComponent))))

(event OnComponentBeginOverlap(GC_)
  (params (OverlappedComponent :type Primitive%20Component%20Object%20Reference) (OtherActor :type Actor%20Object%20Reference) (OtherComp :type Primitive%20Component%20Object%20Reference) (OtherBodyIndex :type Integer) (bFromSweep :type Boolean) (SweepResult :type Hit%20Result%20Structure%20%28by%20ref%29))
  (bind _gc_ (Variables|Default|GetGC_))
  (if (Components|ComponentHasTag OtherComp "FS_MasterField")
    (bind _asbp_master_field (Utilities|Casting|CastToBP_MasterField (Components|GetOwner OtherComp)))
    (if (> (Variables|/Game/Prop/_FiledSystem/BP_MasterField.BP_MasterField_C|GetStrain%20Magnitude _asbp_master_field) (Variables|Default|GetDamageThreshold))
      (Transformation|DetachFromComponent _gc_ "KeepWorld" "KeepWorld" "KeepWorld" true)
      (Physics|SetSimulatePhysics _gc_ true)
      (Collision|SetCollisionProfileName (Variables|Default|GetGC_Collider) "NoCollision" true :!class /Script/Engine.PrimitiveComponent))))

(event EventBeginPlay)

(event Collision|EventActorBeginOverlap
  (params (OtherActor :type Actor%20Object%20Reference)))

(event EventTick
  (params (DeltaSeconds :type Float%20%28single-precision%29)))

(fn ConstructionScript)