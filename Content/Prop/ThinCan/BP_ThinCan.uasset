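; BP_ThinCan is a thin can prop that swaps to a destroyed mesh when hit hard enough.
; Hits use separate impulse thresholds for player-tagged components and others, and only register until the can is converted.
; Overlapping a BP_DelayMasterField's tagged component also destroys it when strain magnitude exceeds a throwing threshold.
; Destruction also updates the GrabManageComponent's grabbed mesh; debug prints expose impulse and strain values.
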(event OnComponentHit(StaticMesh)
  (params (HitComponent :type Primitive%20Component%20Object%20Reference) (OtherActor :type Actor%20Object%20Reference) (OtherComp :type Primitive%20Component%20Object%20Reference) (NormalImpulse :type Vector :default "0, 0, 0") (Hit :type Hit%20Result%20Structure%20%28by%20ref%29))
  (bind _returnvalue (Math|Vector|VectorLength NormalImpulse))
  (if (not (Variables|Default|GetisConverted))
    (if (Components|ComponentHasTag OtherComp "player")
      (if (> _returnvalue (Variables|DamageThreshold|GetHitDamageThreshold))
        (Development|PrintString (Utilities|String|ToString(Float) _returnvalue))
        (Components|StaticMesh|SetStaticMesh (Variables|Default|GetStaticMesh) "/Game/Prop/ThinCan/DT_can/SM_ThinCan_Destroyed.SM_ThinCan_Destroyed" :!label _label)
        (Variables|Default|SetisConverted true)
        (Variables|/Game/Prop/_Base_AllObject/GrabManageComponent.GrabManageComponent_C|SetGrabbedStaticMesh (Variables|Default|GetGrabManageComponent) "/Game/Prop/ThinCan/DT_can/SM_ThinCan_Destroyed.SM_ThinCan_Destroyed"))
      (elif (> (Math|Vector|VectorLength NormalImpulse) (Variables|DamageThreshold|GetCollisionDamageThreshold))
        (goto _label)))))

(event OnComponentBeginOverlap(StaticMesh)
  (params (OverlappedComponent :type Primitive%20Component%20Object%20Reference) (OtherActor :type Actor%20Object%20Reference) (OtherComp :type Primitive%20Component%20Object%20Reference) (OtherBodyIndex :type Integer) (bFromSweep :type Boolean) (SweepResult :type Hit%20Result%20Structure%20%28by%20ref%29))
  (bind _asbp_delay_master_field (Utilities|Casting|CastToBP_DelayMasterField OtherActor))
  (Development|PrintString (Utilities|String|ToString(Float) (Variables|/Game/Prop/_FiledSystem/BP_DelayMasterField.BP_DelayMasterField_C|GetStrain%20Magnitude _asbp_delay_master_field)))
  (if (and (> (Variables|/Game/Prop/_FiledSystem/BP_DelayMasterField.BP_DelayMasterField_C|GetStrain%20Magnitude _asbp_delay_master_field) (Variables|DamageThreshold|GetThrowingDamageThreshold)) (Components|ComponentHasTag OtherComp "FS_MasterField"))
    (Components|StaticMesh|SetStaticMesh (Variables|Default|GetStaticMesh) "/Game/Prop/ThinCan/DT_can/SM_ThinCan_Destroyed.SM_ThinCan_Destroyed")
    (Variables|Default|SetisConverted true)
    (Variables|/Game/Prop/_Base_AllObject/GrabManageComponent.GrabManageComponent_C|SetGrabbedStaticMesh (Variables|Default|GetGrabManageComponent) "/Game/Prop/ThinCan/DT_can/SM_ThinCan_Destroyed.SM_ThinCan_Destroyed")))

(event EventBeginPlay)

(event Collision|EventActorBeginOverlap
  (params (OtherActor :type Actor%20Object%20Reference)))

(event EventTick
  (params (DeltaSeconds :type Float%20%28single-precision%29)))

(fn ConstructionScript)