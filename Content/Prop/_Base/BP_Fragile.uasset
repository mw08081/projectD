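; BP_Fragile is a breakable prop base that shatters into fragments when its state changes from damage.
; ChangeActorState, skipped if already converted, hides the mesh, disables its collision and spawns a BP_FracturedSM per FragileManageComponent mesh.
; Fragment impulses follow the prop's velocity, or the damage causer's if stationary, scaled by mass, causer speed and scattering coefficient.
; The hit event is empty, leaving momentum-based area damage logic disconnected.
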(event OnComponentHit(StaticMesh)
  (params (HitComponent :type Primitive%20Component%20Object%20Reference) (OtherActor :type Actor%20Object%20Reference) (OtherComp :type Primitive%20Component%20Object%20Reference) (NormalImpulse :type Vector :default "0, 0, 0") (Hit :type Hit%20Result%20Structure%20%28by%20ref%29)))

(event EventBeginPlay
  (|CallParentFunction) ; This node is disabled and will not be called.\nDrag off pins to build functionality.
)

(event Collision|EventActorBeginOverlap
  (params (OtherActor :type Actor%20Object%20Reference))
  (|CallParentFunction OtherActor) ; This node is disabled and will not be called.\nDrag off pins to build functionality.
)

(event EventTick
  (params (DeltaSeconds :type Float%20%28single-precision%29))
  (|CallParentFunction DeltaSeconds) ; This node is disabled and will not be called.\nDrag off pins to build functionality.
)

(fn ConstructionScript
  (|CallParentFunction))

(fn ChangeActorState
  (params (Damage :type Float%20%28double-precision%29))
  (bind _returnvalue (Transformation|GetVelocity))
  (bind _returnvalue_2 (Transformation|GetActorTransform))
  (bind _staticmesh (Variables|Default|GetStaticMesh))
  (bind (_location _rotation) (Math|Transform|BreakTransform _returnvalue_2))
  (if (not (Default|GetIsConverted (Variables|Default|GetConvertManageComponent)))
    (|CallParentFunction Damage) ; Fragile은 convertManager에 변경대상이 \n없으므로 딱히 실행안해도됨
    (if (Utilities|Operators|EqualEqual :A _returnvalue :ErrorTolerance 0.001) ; 액터의 속도가없다면, \n부딪힌 액터의 속도를 가져와서 사용
      (LocalVariables|SetLastActorVelocity (Variables|Default|GetDamageCauseLastVelocity))
      (else
        (LocalVariables|SetLastActorVelocity _returnvalue)))
    (if (Variables|Default|GetCanPrintActorVelocity)
      (Development|PrintString (Utilities|String|ToString(Vector) (LocalVariables|GetLastActorVelocity))))
    (Collision|SetCollisionEnabled _staticmesh "NoCollision")
    (Development|SetHiddeninGame _staticmesh true false)
    (for _array_element (Variables|/Game/Prop/_Base/_Base_Component/FragileManageComponent.FragileManageComponent_C|GetStaticMeshes (Variables|Default|GetFragileManageComponent))
      (bind _returnvalue_3 (Game|SpawnActorfromClass "/Game/Prop/_ActionObject/BP_FracturedSM.BP_FracturedSM_C" (Math|Transform|MakeTransform _location _rotation "1.000000,1.000000,1.000000") "AlwaysSpawn" "MultiplyWithRoot" self 0))
      (Components|StaticMesh|SetStaticMesh (Variables|/Game/Prop/_ActionObject/BP_FracturedSM.BP_FracturedSM_C|GetStaticMesh _returnvalue_3) _array_element)
      (Physics|AddImpulse (Variables|/Game/Prop/_ActionObject/BP_FracturedSM.BP_FracturedSM_C|GetStaticMesh _returnvalue_3) (* (Math|Vector|Normalize (LocalVariables|GetLastActorVelocity)) (/ (Physics|GetMass (Variables|/Game/Prop/_ActionObject/BP_FracturedSM.BP_FracturedSM_C|GetStaticMesh _returnvalue_3)) 0.5) (Math|Vector|VectorLength (Variables|Default|GetDamageCauseLastVelocity)) (Variables|/Game/Prop/_Base/_Base_Component/ConvertManageComponent.ConvertManageComponent_C|GetScatteringCoefficient (Variables|Default|GetConvertManageComponent))) "None" false))))