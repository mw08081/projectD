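; Base destructible prop built on a Chaos Geometry Collection that can be grabbed until it fractures.
; The first break event plays a sound, disables grabbing, marks it fractured, and spawns a Niagara effect and floating score priced from LvObjectRoot.
; Overlap by a Bomb-tagged actor spawns a hit effect while unbroken.
; Field-actor overlaps only print strain for debugging, and the collision handler is empty.
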(event OnComponentBeginOverlap(GeometryCollection)
  (params (OverlappedComponent :type Primitive%20Component%20Object%20Reference) (OtherActor :type Actor%20Object%20Reference) (OtherComp :type Primitive%20Component%20Object%20Reference) (OtherBodyIndex :type Integer) (bFromSweep :type Boolean) (SweepResult :type Hit%20Result%20Structure%20%28by%20ref%29))
  ;[1 1 1] Play Hit Ns When overlap by bomb
  (if (and (not (Variables|/Game/Prop/_Base/_Base_Component/FractureManageComponent.FractureManageComponent_C|GetisFractured (Variables|Default|GetFractureManageComponent))) (Actor|ActorHasTag OtherActor "Bomb"))
    (Default|SpawnHitNsatLocation (Variables|Default|GetBP_Gameinstance) (Transformation|GetActorLocation))))

(event OnComponentHit(GeometryCollection)
  (params (HitComponent :type Primitive%20Component%20Object%20Reference) (OtherActor :type Actor%20Object%20Reference) (OtherComp :type Primitive%20Component%20Object%20Reference) (NormalImpulse :type Vector :default "0, 0, 0") (Hit :type Hit%20Result%20Structure%20%28by%20ref%29)))

(event Custom|ChaosCollisionEvent
  (params (CollisionInfo :type Chaos%20Physics%20Collision%20Info%20Structure%20%28by%20ref%29)))

(event Custom|ChaosBreakEvent
  (params (BreakEvent :type Chaos%20Break%20Event%20Structure%20%28by%20ref%29))
  (Utilities|FlowControl|DoOnce false
    (:Completed
      (Default|PlaySfx (Variables|Default|GetSfxPlayComponent) "NewEnumerator0")
      (if (not (Variables|/Game/Prop/_Base/_Base_Component/FractureManageComponent.FractureManageComponent_C|GetisFractured (Variables|Default|GetFractureManageComponent)))
        ;[1 1 1] Change object state(ex cant be grabbed)
        (Default|SetCanGrab (Variables|Default|GetGrabManageComponent) false)
        (Variables|/Game/Prop/_Base/_Base_Component/FractureManageComponent.FractureManageComponent_C|SetisFractured (Variables|Default|GetFractureManageComponent) true)
        ;[1 1 1] GAME INSTANCE
        (bind _asbp_game_instance (Utilities|Casting|CastToBP_GameInstance (Game|GetGameInstance)))
        (bind _ns (Default|GetNsfromENSCode _asbp_game_instance (Variables|/Game/Prop/_Base/_Base_Component/FractureManageComponent.FractureManageComponent_C|GetENSCode (Variables|Default|GetFractureManageComponent))))
        (Default|SpawnNsatLocation _asbp_game_instance _ns (.location BreakEvent))
        ;[1 1 1] Game mode
        (bind _asbp_project_d_default_game_mode (Utilities|Casting|CastToBP_ProjectD_DefaultGameMode (Game|GetGameMode)))
        (Class|ProjectDDefaultGameMode|SpawnFloatingScore _asbp_project_d_default_game_mode (Transformation|GetActorLocation) (Variables|/Script/ProjectD.LvObjectRoot|GetobjectPrice (Variables|Default|GetLvObjectRoot)))))))

(event EventBeginPlay
  (bind _geometrycollection (Variables|Default|GetGeometryCollection))
  (EventDispatchers|BindEventtoOnChaosPhysicsCollision _geometrycollection (EventDispatchers|CreateEvent :!event Custom|ChaosCollisionEvent))
  (EventDispatchers|BindEventtoOnChaosBreakEvent _geometrycollection (EventDispatchers|CreateEvent :!event Custom|ChaosBreakEvent))
  (Default|SetGrabbedObjectMass (Variables|Default|GetGrabManageComponent) (Variables|Default|GetGC_Mass)))

(event Collision|EventActorBeginOverlap
  (params (OtherActor :type Actor%20Object%20Reference))
  (bind _asbp_delay_master_field (Utilities|Casting|CastToBP_DelayMasterField OtherActor))
  (Development|PrintString (Utilities|String|Append (Utilities|String|ToString(Float) (Variables|/Game/_FiledSystem/BP_DelayMasterField.BP_DelayMasterField_C|GetStrain%20Magnitude _asbp_delay_master_field)) " power overlaped")))

(fn ConstructionScript)