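; Deprecated base Blueprint for a grabbable Chaos Geometry Collection prop that shatters and awards score from its object price.
; On break it plays a sound and, the first time, disables grabbing, marks itself fractured, spawns effects from FractureManageComponent codes via the game instance, then scores after a delay.
; Bomb-tagged overlaps spawn a hit effect while intact, and damage events only print debug text.
; ApplyExternalStrainMagnitude applies a huge strain at the actor's location to force fracture.
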(event OnComponentBeginOverlap(GeometryCollection)
  (params (OverlappedComponent :type Primitive%20Component%20Object%20Reference) (OtherActor :type Actor%20Object%20Reference) (OtherComp :type Primitive%20Component%20Object%20Reference) (OtherBodyIndex :type Integer) (bFromSweep :type Boolean) (SweepResult :type Hit%20Result%20Structure%20%28by%20ref%29))
  ;[1 1 1] Play Hit Ns When overlap by bomb
  (if (and (not (Variables|/Game/Prop/_Base/_Base_Component/FractureManageComponent.FractureManageComponent_C|GetisFractured (Variables|Default|GetFractureManageComponent))) (Actor|ActorHasTag OtherActor "Bomb"))
    (Default|SpawnHitNsatLocation (Variables|Default|GetBP_Gameinstance) (Transformation|GetActorLocation))))

(event Custom|ChaosCollisionEvent
  (params (CollisionInfo :type Chaos%20Physics%20Collision%20Info%20Structure%20%28by%20ref%29)))

(event Custom|OnTakeAnyDamage_Event
  (params (DamagedActor :type Actor%20Object%20Reference) (Damage :type Float%20%28single-precision%29) (DamageType :type Damage%20Type%20Object%20Reference) (InstigatedBy :type Controller%20Object%20Reference) (DamageCauser :type Actor%20Object%20Reference))
  (Development|PrintString (Utilities|String|Append (Utilities|GetDisplayName DamagedActor) "가 피격됨(" "(" (Utilities|GetDisplayName DamageCauser) "의한 데미지:" (Utilities|String|ToString(Float) Damage) ")")))

(event Custom|ChaosBreakEvent
  (params (BreakEvent :type Chaos%20Break%20Event%20Structure%20%28by%20ref%29))
  (Utilities|FlowControl|DoOnce false :!label _label
    (:Completed
      (Default|PlaySfx (Variables|Default|GetSfxPlayComponent) "NewEnumerator0")
      (if (not (Variables|/Game/Prop/_Base/_Base_Component/FractureManageComponent.FractureManageComponent_C|GetisFractured (Variables|Default|GetFractureManageComponent)))
        ;[1 1 1] Change object state(ex cant be grabbed)
        (Default|SetCanGrab (Variables|Default|GetGrabManageComponent) false)
        (Variables|/Game/Prop/_Base/_Base_Component/FractureManageComponent.FractureManageComponent_C|SetisFractured (Variables|Default|GetFractureManageComponent) true)
        ;[1 1 1] GAME INSTANCE
        (bind _asbp_game_instance (Utilities|Casting|CastToBP_GameInstance (Game|GetGameInstance)))
        (for _array_element (Variables|/Game/Prop/_Base/_Base_Component/FractureManageComponent.FractureManageComponent_C|GetENSCode (Variables|Default|GetFractureManageComponent))
          (bind _ns (Default|GetNsfromENSCode _asbp_game_instance _array_element))
          (Default|SpawnNsatLocation _asbp_game_instance _ns (.location BreakEvent))
          (bind _asproject_d_default_game_mode (Utilities|Casting|CastToProjectD_DefaultGameMode (Game|GetGameMode)))
          (Utilities|FlowControl|Delay 2.0)
          (Class|ProjectDDefaultGameMode|GetScore _asproject_d_default_game_mode (Variables|/Script/ProjectD.LvObjectRoot|GetobjectPrice (Variables|Default|GetLvObjectRoot)))
          (goto _label Reset))))))

(event EventBeginPlay
  (bind _geometrycollection (Variables|Default|GetGeometryCollection))
  (bind _geometrycollection_2 (Variables|Default|GetGeometryCollection))
  (EventDispatchers|BindEventtoOnChaosPhysicsCollision _geometrycollection (EventDispatchers|CreateEvent :!event Custom|ChaosCollisionEvent))
  (EventDispatchers|BindEventtoOnChaosBreakEvent _geometrycollection (EventDispatchers|CreateEvent :!event Custom|ChaosBreakEvent))
  (Default|SetGrabbedObjectMass (Variables|Default|GetGrabManageComponent) (Variables|Default|GetGC_Mass))
  (Collision|SetCollisionResponsetoChannel _geometrycollection_2 "ECC_Pawn" "ECR_Overlap")
  (Collision|SetCollisionObjectType _geometrycollection_2 "ECC_Destructible"))

(fn ConstructionScript)

(fn ApplyExternalStrainMagnitude
  (Class|GeometryCollectionComponent|ApplyExternalStrain (Variables|Default|GetGeometryCollection) 0 (Transformation|GetActorLocation) 1e+02 0 1.0 1111111111111.0))