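; Back cushion prop (variant C) for the big interior sofa, with grab support through its GrabManageComponent.
; Tick runs the parent logic, then draws debug spheres at the actor origin and at the component's GrabPivot, converted from local to world space.
; The construction script only calls the parent, and a GrabHandle setter sits unconnected in the event graph.
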(event EventBeginPlay
  (|CallParentFunction) ; This node is disabled and will not be called.\nDrag off pins to build functionality.
)

(event Collision|EventActorBeginOverlap
  (params (OtherActor :type Actor%20Object%20Reference))
  (|CallParentFunction OtherActor) ; This node is disabled and will not be called.\nDrag off pins to build functionality.
)

(event EventTick
  (params (DeltaSeconds :type Float%20%28single-precision%29))
  (|CallParentFunction DeltaSeconds)
  (Rendering|Debug|DrawDebugSphere (Transformation|GetActorLocation) 5.0 12 "(R=1.000000,G=1.000000,B=1.000000,A=1.000000)" 0.0)
  (Rendering|Debug|DrawDebugSphere (Math|Transform|TransformLocation (Transformation|GetActorTransform) (Variables|/Game/Prop/_Base/_Base_Component/GrabManageComponent.GrabManageComponent_C|GetGrabPivot (Variables|Default|GetGrabManageComponent))) 1e+01 12 "(R=1.000000,G=0.000000,B=0.488189,A=1.000000)" 0.0))

(fn ConstructionScript
  (|CallParentFunction))