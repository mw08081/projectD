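; BP_Test_Paper is a test actor that gives paper-flutter feedback when the player bumps into it.
; Its StaticMesh hit event checks for the "player" component tag, plays a fluttering sound at the impact point, and spawns a BP_NsObject there set to the paper particle.
; An IsTest flag held through a short Delay throttles repeated hits.
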(event OnComponentHit(StaticMesh)
  (params (HitComponent :type Primitive%20Component%20Object%20Reference) (OtherActor :type Actor%20Object%20Reference) (OtherComp :type Primitive%20Component%20Object%20Reference) (NormalImpulse :type Vector :default "0, 0, 0") (Hit :type Hit%20Result%20Structure%20%28by%20ref%29))
  (if (not (Variables|Default|GetisTest))
    (if (Components|ComponentHasTag OtherComp "player")
      (Variables|Default|SetisTest true)
      (Audio|PlaySoundatLocation "/Game/System/Sound/soundEffect/paper_fluttering.paper_fluttering" (.impactpoint Hit) "0, 0, 0" 1.0 1.0 0.0 0 0 0 0)
      (bind _returnvalue (Game|SpawnActorfromClass "/Game/Prop/_ActionObject/BP_NsObject.BP_NsObject_C" (Math|Conversions|ToTransform(Vector) (.impactpoint Hit)) "Undefined" "MultiplyWithRoot" 0 0))
      (Default|SetNs _returnvalue "/Game/StarterContent/VFX/02-1/Particle_Paper.Particle_Paper")
      (Utilities|FlowControl|Delay 0.2)
      (Variables|Default|SetisTest false))))

(event EventBeginPlay)

(event Collision|EventActorBeginOverlap
  (params (OtherActor :type Actor%20Object%20Reference)))

(event EventTick
  (params (DeltaSeconds :type Float%20%28single-precision%29)))

(fn ConstructionScript)