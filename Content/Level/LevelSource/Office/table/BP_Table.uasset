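; BP_Table is a grabbable, destructible office table with a price reported to the game instance.
; On BeginPlay it feeds its mesh and mass to GrabManageComponent and registers its price.
; Overlap with a bomb field, or a master or delayed master field straining above ConvertManageComponent's threshold, triggers a sound lookup and one-time conversion.
; Conversion swaps in random destroyed meshes, spawns Niagara effects and reports destruction through the game instance.
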(event OnComponentBeginOverlap(StaticMesh)
  (params (OverlappedComponent :type Primitive%20Component%20Object%20Reference) (OtherActor :type Actor%20Object%20Reference) (OtherComp :type Primitive%20Component%20Object%20Reference) (OtherBodyIndex :type Integer) (bFromSweep :type Boolean) (SweepResult :type Hit%20Result%20Structure%20%28by%20ref%29))
  (bind _convertmanagecomponent (Variables|Default|GetConvertManageComponent))
  (bind _dmgthreshold (Variables|/Game/Prop/_Base_Component/ConvertManageComponent.ConvertManageComponent_C|GetDmgThreshold _convertmanagecomponent))
  (bind _asbp_master_field (Utilities|Casting|CastToBP_MasterField OtherActor)
    (:then
      (if (> (Variables|/Game/Prop/_FiledSystem/BP_MasterField.BP_MasterField_C|GetStrain%20Magnitude _asbp_master_field) _dmgthreshold)
        (bind _bp_gameinstance (CallFunction|PlayConvertEventSound :!label _label))
        (if (not (Variables|/Game/Prop/_Base_Component/ConvertManageComponent.ConvertManageComponent_C|GetisConverted (Variables|Default|GetConvertManageComponent)))
          (CallFunction|ChangeActorState)
          (bind _ns (Default|GetNsfromENSCode _bp_gameinstance (Variables|/Game/Prop/_Base_Component/ConvertManageComponent.ConvertManageComponent_C|GetEvent_ENSCode (Variables|Default|GetConvertManageComponent))))
          (Default|SpawnNsatLocation _bp_gameinstance _ns (Transformation|GetActorLocation))
          (CallFunction|EventDestroy _bp_gameinstance))))
    (:CastFailed
      (bind _asbp_delay_master_field (Utilities|Casting|CastToBP_DelayMasterField OtherActor)
        (:then
          (if (> (Variables|/Game/Prop/_FiledSystem/BP_DelayMasterField.BP_DelayMasterField_C|GetStrain%20Magnitude _asbp_delay_master_field) _dmgthreshold)
            (goto _label)))
        (:CastFailed
          (Utilities|Casting|CastToBP_BombField OtherActor)
          (goto _label))))))

(event EventBeginPlay
  (bind _staticmesh (Variables|Default|GetStaticMesh))
  (bind _grabmanagecomponent (Variables|Default|GetGrabManageComponent))
  (Default|SetGrabbedStaticMesh _grabmanagecomponent (Variables|/Script/Engine.StaticMeshComponent|GetStaticMesh _staticmesh))
  (Default|SetGrabbedObjectMass _grabmanagecomponent (Physics|GetMass _staticmesh))
  (bind _asbp_game_instance (Utilities|Casting|CastToBP_GameInstance (Game|GetGameInstance)))
  (Default|CalcObjPrice _asbp_game_instance (Variables|/Script/ProjectD.LvObjectRoot|GetobjectPrice (Variables|Default|GetLvObjectRoot))))

(fn ConstructionScript)

(fn ChangeActorState
  (bind _convertmanagecomponent (Variables|Default|GetConvertManageComponent))
  (bind _destroyed_tartget_staticmesh (Variables|/Game/Prop/_Base_Component/ConvertManageComponent.ConvertManageComponent_C|GetDESTROYED_TARTGET_STATICMESH _convertmanagecomponent))
  (bind _outitem (Utilities|Array|Random _destroyed_tartget_staticmesh))
  ;[1 1 1] Change State
  (Variables|/Game/Prop/_Base_Component/ConvertManageComponent.ConvertManageComponent_C|SetisConverted (Variables|Default|GetConvertManageComponent) true)
  (if (> (Utilities|Array|Length _destroyed_tartget_staticmesh) 0)
    (Components|StaticMesh|SetStaticMesh (Variables|Default|GetStaticMesh) _outitem)
    (Default|SetGrabbedStaticMesh (Variables|Default|GetGrabManageComponent) _outitem)))

(fn PlayConvertEventSound
  (bind _asbp_game_instance (Utilities|Casting|CastToBP_GameInstance (Game|GetGameInstance)))
  (Default|GetSoundbyESwCode _asbp_game_instance (Variables|/Game/Prop/_Base_Component/ConvertManageComponent.ConvertManageComponent_C|GetEvent_ESWCode (Variables|Default|GetConvertManageComponent)))
  (return _asbp_game_instance))

(fn EventDestroy
  (params (BP_GameInstance :type BP%20Game%20Instance%20Object%20Reference))
  (Default|EventDestroy BP_GameInstance (Variables|/Script/ProjectD.LvObjectRoot|GetobjectPrice (Variables|Default|GetLvObjectRoot))))

(fn PlayAfterConvertingCollisionSound)